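; SuperJumpBP is an actor Blueprint for a super jump, though as wired it only plays an explosion effect.
; Pressing the right mouse button spawns the P_Explosion emitter at the player character's location, with auto-destroy off.
; An upward force on the player's capsule is left unconnected and never runs, so no jump occurs.
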(event EventBeginPlay)

(event Collision|EventActorBeginOverlap
  (params (OtherActor :type Actor%20Object%20Reference)))

(event EventTick
  (params (DeltaSeconds :type Float%20%28single-precision%29)))

(event Input|MouseEvents|RightMouseButton
  (params (Key :type Key%20Structure :default "AnyKey"))
  (:Pressed
    (Effects|SpawnEmitteratLocation "/Game/StarterContent/Particles/P_Explosion.P_Explosion" (Transformation|GetActorLocation (Game|GetPlayerCharacter 0)) "0, 0, 0" false)))

(fn ConstructionScript)